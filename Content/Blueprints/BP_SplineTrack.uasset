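; BP_SplineTrack is a spline-based track that returns itself as a grind rail through GetGrindRail.
; Its construction script tiles spline mesh components along the spline, spacing them by the mesh's X bounding-box length.
; Each segment takes local positions and tangents from the spline, with tangents clamped to segment length to match the tiling.
; Segments share one material and receive their color through custom primitive data.
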(fn `GetGrindRail`
  (returns (GrindRail :type "/Game/Blueprints/BP_SplineTrack Object Reference"))
  (return self))

(fn `UserConstructionScript`
  (bind (_cpdcolor_r _cpdcolor_g _cpdcolor_b) (break `LinearColor` (`self.CPDColor`)))
  (bind _spline (`self.Spline`))
  (bind _spline_2 (`self.Spline`))
  (bind (_returnvalue_min _returnvalue_max) (break `Box` (`StaticMesh.GetBoundingBox` (`self.Mesh`))))
  (bind _returnvalue_x (`KismetMathLibrary.BreakVector` (+ (`KismetMathLibrary.Vector_GetAbs` _returnvalue_min) (`KismetMathLibrary.Vector_GetAbs` _returnvalue_max))))
  (bind _output_get (set `self.XLength` _returnvalue_x))
  (for _index (range (+ (`KismetMathLibrary.FTrunc` (/ (`SplineComponent.GetSplineLength` (`self.Spline`)) _output_get)) 1))
    (bind _returnvalue (`AddComponent|NODE_AddSplineMeshComponent-0`))
    (bind _output_get_2 (set `self.SplineMesh` _returnvalue))
    (`StaticMeshComponent.SetStaticMesh` _output_get_2 (`self.Mesh`))
    (bind _returnvalue_2 (* _index (`self.XLength`)))
    (bind _returnvalue_3 (* (+ _index 1) (`self.XLength`)))
    (`SplineMeshComponent.SetStartAndEnd` _output_get_2 (`SplineComponent.GetLocationAtDistanceAlongSpline` _spline_2 _returnvalue_2 "Local") (`KismetMathLibrary.ClampVectorSize` (`SplineComponent.GetTangentAtDistanceAlongSpline` _spline_2 _returnvalue_2 "Local") 0.0 (`self.XLength`)) (`SplineComponent.GetLocationAtDistanceAlongSpline` _spline _returnvalue_3 "Local") (`KismetMathLibrary.ClampVectorSize` (`SplineComponent.GetTangentAtDistanceAlongSpline` _spline _returnvalue_3 "Local") 0.0 (`self.XLength`)) true)
    (`PrimitiveComponent.SetMaterial` _output_get_2 0 (`self.Material`))
    (`PrimitiveComponent.SetDefaultCustomPrimitiveDataVector3` (`self.SplineMesh`) 0 (`KismetMathLibrary.MakeVector` _cpdcolor_r _cpdcolor_g _cpdcolor_b))))