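; BP_Lego is a Blueprint actor that plays a plastic impact sound on hard collisions.
; Its StaticMesh hit event checks whether either the other component's velocity or the actor's own velocity exceeds a speed threshold.
; A DoOnce gate, reset after a short delay, rate-limits the non-spatialized 2D sound so repeated hits do not spam audio.
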(event `self.StaticMesh.OnComponentHit`
  (params (HitComponent :type "PrimitiveComponent Object Reference") (OtherActor :type "Actor Object Reference") (OtherComp :type "PrimitiveComponent Object Reference") (NormalImpulse :type "Vector Structure") (Hit :type "HitResult Structure (by ref)"))
  (if (or (> (`KismetMathLibrary.VSize` (`SceneComponent.GetComponentVelocity` OtherComp)) 1000.0) (> (`KismetMathLibrary.VSize` (`self.GetVelocity`)) 1000.0))
    (`/Engine/EditorBlueprintResources/StandardMacros.DoOnce` false :!label _label
      (:`Completed`
        (`GameplayStatics.PlaySound2D` "/Game/Audio/PlasticHit/SC_PlasticHit.SC_PlasticHit" 1.0 1.0 0.0 null null)
        (`KismetSystemLibrary.Delay` 1.0)
        (goto _label :!via `Reset`)))))

(fn `UserConstructionScript`)