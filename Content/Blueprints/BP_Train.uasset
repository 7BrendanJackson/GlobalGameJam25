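; BP_Train is a train actor that runs continuously along the spline of a referenced SplineActor.
; On BeginPlay it turns its static mesh components into a carriage list, stacking each one's trailing offset from its mesh X bounds, slightly shortened.
; Tick advances a shared distance by Speed and places each carriage at that distance minus its offset, matching spline location and rotation and wrapping by modulo of the spline length.
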(event `self.ReceiveBeginPlay`
  (bind _carriages (`self.Carriages`))
  (bind _splineactor (`self.SplineActor`)
    (:`then`
      (bind _output_get (set `self.Spline` (`/Game/Blueprints/BP_TrainTrack.Spline` _splineactor)))
      (set `self.TotalLength` (`SplineComponent.GetSplineLength` _output_get))
      (`|ExecutionSequence`
        (:`then_0`
          (for (_array_element _array_index) (`self.K2_GetComponentsByClass` "/Script/Engine.StaticMeshComponent")
            (if (== _array_index 0)
              (bind (_min _max) (`StaticMeshComponent.GetLocalBounds` _array_element))
              (bind _returnvalue (- (- (.x _max) (.x _min)) 2.5))
              (`KismetArrayLibrary.Array_Add` (`self.Carriages`) (make `/Game/TrainCarriages` _array_element _returnvalue))
              (else
                (bind (_output_carriage _output_length _output_position) (break `/Game/TrainCarriages` (`|GetArrayItem` _carriages (- _array_index 1))))
                (`KismetArrayLibrary.Array_Add` _carriages (make `/Game/TrainCarriages` _array_element _returnvalue (+ _output_position _returnvalue)))))))
        (:`then_1`
          (set `self.Time` (`self.TotalLength`)))))
    (:`else`)))

(event `self.ReceiveTick`
  (params (DeltaSeconds :type "Float (single-precision)"))
  (bind _spline (`self.Spline`))
  (bind _output_get (set `self.Time` (+ (`self.Time`) (* DeltaSeconds (`self.Speed`)))))
  (for _array_element (`self.Carriages`)
    (bind _returnvalue (mod (- _output_get (`.Position_7_498064ED48CB7AFB2CB7F58342CDC599` (break `/Game/TrainCarriages` _array_element))) (`self.TotalLength`)))
    (`SceneComponent.K2_SetWorldLocationAndRotation` (break `/Game/TrainCarriages` _array_element) (`SplineComponent.GetLocationAtDistanceAlongSpline` _spline _returnvalue "World") (`SplineComponent.GetRotationAtDistanceAlongSpline` _spline _returnvalue "World") false false)))

(fn `UserConstructionScript`)