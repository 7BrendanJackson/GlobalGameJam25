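; Toggleable boost pad that launches a hamster along its arrow's direction when the hamster is in bubble state.
; A sphere overlap queries BPI_Hamster and boosts only when powered and the normalized, ground-projected velocity aligns enough with the pad's forward vector, followed by a brief recharge.
; ChangePowerState, also bound to debug key G, runs a timeline that fades the decal's alpha and updates Powered.
; The construction script sets the initial decal visibility from Powered.
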(event OnComponentBeginOverlap(Sphere)
  (params (OverlappedComponent :type Primitive%20Component%20Object%20Reference) (OtherActor :type Actor%20Object%20Reference) (OtherComp :type Primitive%20Component%20Object%20Reference) (OtherBodyIndex :type Integer) (bFromSweep :type Boolean) (SweepResult :type Hit%20Result%20Structure%20%28by%20ref%29))
  (if (and (not (Variables|Default|GetRecharging)) (Variables|Default|GetPowered))
    (if (Utilities|DoesObjectImplementInterface OtherActor "/Game/Blueprints/BPI_Hamster.BPI_Hamster_C")
      (bind _hamster (Class|BPIHamster|GetHampster(Message) OtherActor))
      (if (Variables|/Game/Characters/BP_Hamster.BP_Hamster_C|GetIsBubble? _hamster)
        (if (> (Math|Vector|DotProduct (Transformation|GetActorForwardVector) (Math|Vector|ProjectVectorontoPlane (Math|Vector|Normalize (Transformation|GetVelocity _hamster)) "0.000000,0.000000,1.000000")) (Variables|Default|GetBoostDot))
          (Variables|Default|SetRecharging true)
          (Default|Boost _hamster (Variables|Default|GetBoostSpeed) (Math|Vector|GetForwardVector (Variables|Default|GetArrow)))
          (Utilities|FlowControl|Delay 0.2)
          (Variables|Default|SetRecharging false))))))

(event Custom|ChangePowerState
  (params (PowerState :type Boolean))
  (if (not (== PowerState (Variables|Default|GetPowered)))
    (if PowerState
      (bind _poweralpha (Timeline|PowerTransition Play)
        (:Update
          (Rendering|Components|Decal|SetDecalColor (Variables|Default|GetDecal) (Utilities|Struct|MakeLinearColor 0.0 0.0 0.0 _poweralpha)))
        (:Finished
          (Variables|Default|SetPowered PowerState)))
      (else
        (Timeline|PowerTransition Reverse)))))

(event Input|KeyboardEvents|DebugKeyG
  (params (Key :type Key%20Structure :default "None") (ActionValue :type Input%20Action%20Value%20Structure))
  (:Pressed
    (CallFunction|ChangePowerState (not (Variables|Default|GetPowered)))))

(fn ConstructionScript
  (Rendering|Components|Decal|SetDecalColor (Variables|Default|GetDecal) (Utilities|Struct|MakeLinearColor 0.0 0.0 0.0 (select (Variables|Default|GetPowered) 1.0 0.0))))