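; BP_TV is a TV actor that toggles the MPC_Dark material parameter collection between inside-TV and outside-TV states.
; Flip writes the OutSideTV scalar as 0 or 1 from the Inside flag, while SetTVSide always sets it to 0.
; The Box end-overlap handler only casts to Character.
; A dot-product side test that would set Inside and call Flip is disconnected, with empty vector inputs.
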(event `self.ReceiveTick`
  (params (DeltaSeconds :type "Float (single-precision)"))
  (if true
    _))

(event `self.Box.OnComponentEndOverlap`
  (params (OverlappedComponent :type "PrimitiveComponent Object Reference") (OtherActor :type "Actor Object Reference") (OtherComp :type "PrimitiveComponent Object Reference") (OtherBodyIndex :type Integer))
  (cast `Character` OtherActor))

(event `Flip`
  (if (`self.Inside?`)
    (`KismetMaterialLibrary.SetScalarParameterValue` "/Game/VFX/MPC_Dark.MPC_Dark" "OutSideTV" 0.0)
    (else
      (`KismetMaterialLibrary.SetScalarParameterValue` "/Game/VFX/MPC_Dark.MPC_Dark" "OutSideTV" 1.0))))

(fn `SetTVSide`
  (`KismetMaterialLibrary.SetScalarParameterValue` "/Game/VFX/MPC_Dark.MPC_Dark" "OutSideTV"))

(fn `UserConstructionScript`)