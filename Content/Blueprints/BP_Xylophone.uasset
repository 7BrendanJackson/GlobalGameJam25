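; BP_Xylophone is a playable xylophone with seven key components that each play a note when an actor begins overlapping them.
; All keys share the SC_Xylophone sound, using a fixed pitch multiplier per key that rises from Key7 to Key1.
; The overlapping actor's speed sets the volume, with Key7 using a wider speed range than the others.
; Every note plays at Key7's world location.
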(event `self.Key7.OnComponentBeginOverlap`
  (params (OverlappedComponent :type "PrimitiveComponent Object Reference") (OtherActor :type "Actor Object Reference") (OtherComp :type "PrimitiveComponent Object Reference") (OtherBodyIndex :type Integer) (bFromSweep :type Boolean) (SweepResult :type "HitResult Structure (by ref)"))
  (set `self.Pitch` 0.5)
  (set `self.Location` (`SceneComponent.K2_GetComponentLocation` (`self.Key7`)))
  (set `self.Volume` (`KismetMathLibrary.MapRangeClamped` (`KismetMathLibrary.VSize` (`self.GetVelocity` OtherActor)) 0.0 2000.0 0.0 1.0))
  (`GameplayStatics.PlaySoundAtLocation` "/Game/Audio/Xylophone/SC_Xylophone.SC_Xylophone" (`self.Location`) (struct) (`self.Volume`) (`self.Pitch`) 0.0 null null null null))

(event `self.Key6.OnComponentBeginOverlap`
  (params (OverlappedComponent :type "PrimitiveComponent Object Reference") (OtherActor :type "Actor Object Reference") (OtherComp :type "PrimitiveComponent Object Reference") (OtherBodyIndex :type Integer) (bFromSweep :type Boolean) (SweepResult :type "HitResult Structure (by ref)"))
  (`GameplayStatics.PlaySoundAtLocation` "/Game/Audio/Xylophone/SC_Xylophone.SC_Xylophone" (`SceneComponent.K2_GetComponentLocation` (`self.Key7`)) (struct) (`KismetMathLibrary.MapRangeClamped` (`KismetMathLibrary.VSize` (`self.GetVelocity` OtherActor)) 0.0 1000.0 0.0 1.0) 0.714 0.0 null null null null))

(event `self.Key5.OnComponentBeginOverlap`
  (params (OverlappedComponent :type "PrimitiveComponent Object Reference") (OtherActor :type "Actor Object Reference") (OtherComp :type "PrimitiveComponent Object Reference") (OtherBodyIndex :type Integer) (bFromSweep :type Boolean) (SweepResult :type "HitResult Structure (by ref)"))
  (`GameplayStatics.PlaySoundAtLocation` "/Game/Audio/Xylophone/SC_Xylophone.SC_Xylophone" (`SceneComponent.K2_GetComponentLocation` (`self.Key7`)) (struct) (`KismetMathLibrary.MapRangeClamped` (`KismetMathLibrary.VSize` (`self.GetVelocity` OtherActor)) 0.0 1000.0 0.0 1.0) 0.928 0.0 null null null null))

(event `self.Key4.OnComponentBeginOverlap`
  (params (OverlappedComponent :type "PrimitiveComponent Object Reference") (OtherActor :type "Actor Object Reference") (OtherComp :type "PrimitiveComponent Object Reference") (OtherBodyIndex :type Integer) (bFromSweep :type Boolean) (SweepResult :type "HitResult Structure (by ref)"))
  (`GameplayStatics.PlaySoundAtLocation` "/Game/Audio/Xylophone/SC_Xylophone.SC_Xylophone" (`SceneComponent.K2_GetComponentLocation` (`self.Key7`)) (struct) (`KismetMathLibrary.MapRangeClamped` (`KismetMathLibrary.VSize` (`self.GetVelocity` OtherActor)) 0.0 1000.0 0.0 1.0) 1.357 0.0 null null null null))

(event `self.Key3.OnComponentBeginOverlap`
  (params (OverlappedComponent :type "PrimitiveComponent Object Reference") (OtherActor :type "Actor Object Reference") (OtherComp :type "PrimitiveComponent Object Reference") (OtherBodyIndex :type Integer) (bFromSweep :type Boolean) (SweepResult :type "HitResult Structure (by ref)"))
  (`GameplayStatics.PlaySoundAtLocation` "/Game/Audio/Xylophone/SC_Xylophone.SC_Xylophone" (`SceneComponent.K2_GetComponentLocation` (`self.Key7`)) (struct) (`KismetMathLibrary.MapRangeClamped` (`KismetMathLibrary.VSize` (`self.GetVelocity` OtherActor)) 0.0 1000.0 0.0 1.0) 1.65 0.0 null null null null))

(event `self.Key2.OnComponentBeginOverlap`
  (params (OverlappedComponent :type "PrimitiveComponent Object Reference") (OtherActor :type "Actor Object Reference") (OtherComp :type "PrimitiveComponent Object Reference") (OtherBodyIndex :type Integer) (bFromSweep :type Boolean) (SweepResult :type "HitResult Structure (by ref)"))
  (`GameplayStatics.PlaySoundAtLocation` "/Game/Audio/Xylophone/SC_Xylophone.SC_Xylophone" (`SceneComponent.K2_GetComponentLocation` (`self.Key7`)) (struct) (`KismetMathLibrary.MapRangeClamped` (`KismetMathLibrary.VSize` (`self.GetVelocity` OtherActor)) 0.0 1000.0 0.0 1.0) 2.0 0.0 null null null null))

(event `self.Key1.OnComponentBeginOverlap`
  (params (OverlappedComponent :type "PrimitiveComponent Object Reference") (OtherActor :type "Actor Object Reference") (OtherComp :type "PrimitiveComponent Object Reference") (OtherBodyIndex :type Integer) (bFromSweep :type Boolean) (SweepResult :type "HitResult Structure (by ref)"))
  (`GameplayStatics.PlaySoundAtLocation` "/Game/Audio/Xylophone/SC_Xylophone.SC_Xylophone" (`SceneComponent.K2_GetComponentLocation` (`self.Key7`)) (struct) (`KismetMathLibrary.MapRangeClamped` (`KismetMathLibrary.VSize` (`self.GetVelocity` OtherActor)) 0.0 1000.0 0.0 1.0) 2.5 0.0 null null null null))

(fn `UserConstructionScript`)